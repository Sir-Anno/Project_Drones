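; Health component that tracks an owner's health and broadcasts damage, health changes and death through event dispatchers.
; BeginPlay stores the starting Health as MaxHealth and announces full health.
; TakeDamage broadcasts the damage and passes reduced health to UpdateHealth, which broadcasts value and clamped percentage, then runs DeathCheck.
; DeathCheck broadcasts Killed whenever health is zero or below, and UpdateHealth broadcasts it again behind a DoOnce.
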(event `self.ReceiveBeginPlay`
  (bind _health (`self.Health`))
  (set `self.MaxHealth` _health)
  (`self.ED_HealthUpdated` _health 1.0))

(fn `Take damage`
  (params (`Damage taken` :type "Float (double-precision)"))
  (`self.ED_DamageTaken` `Damage taken`)
  (`self.Update health` (- (`self.Health`) `Damage taken`)))

(fn `Update health`
  (params (`New health` :type "Float (double-precision)"))
  (bind _output_get (set `self.Health` `New health`))
  (bind _output_get_2 (set `self.Health percentage` (`KismetMathLibrary.MapRangeClamped` (`self.Health`) 0.0 (`self.MaxHealth`) 0.0 1.0)))
  (`self.ED_HealthUpdated` _output_get _output_get_2)
  (`self.Death check`
    (:`Is dead`
      (`/Engine/EditorBlueprintResources/StandardMacros.DoOnce` false
        (:`Completed`
          (`self.ED_Killed`))))))