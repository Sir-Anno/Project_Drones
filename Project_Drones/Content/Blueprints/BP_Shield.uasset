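; Drone shield actor with its own health pool that breaks under damage and comes back after a delay.
; Damage lowers Health and feeds the remaining fraction into a dynamic material parameter on the shield sphere.
; At zero health the sphere is hidden and actor collision is disabled, then a one-shot timer restores full health, visibility and collision.
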(event `self.ReceiveBeginPlay`
  ;[0.1 0.1 0.1] Create matieral instance
  (bind _returnvalue (`PrimitiveComponent.CreateDynamicMaterialInstance` (`self.Sphere`) 0 "/Game/Assets/Materials/M_DroneShield.M_DroneShield" "None"))
  (set `self.Shield material` _returnvalue))

(event `self.ReceiveAnyDamage`
  (params (Damage :type "Float (single-precision)") (DamageType :type "DamageType Object Reference") (InstigatedBy :type "Controller Object Reference") (DamageCauser :type "Actor Object Reference"))
  ;[0.1 0.1 0.1] Take damage
  (`self.TakeDamage` Damage)
  (`self.Update shield material`)
  (`self.Check shield down`
    (:`Shield down`
      (`self.Enable shield` false)
      (`self.Start shield recharge`))))

(event `Start shield recharge`
  ;[0.1 0.1 0.1] Recharge shield
  (`KismetSystemLibrary.K2_SetTimerDelegate` (delegate `Recharge shield`) (`self.Shield recharge time`)))

(event `Recharge shield`
  ;[0.1 0.1 0.1] Recharge shield
  (`self.Enable shield` true)
  (set `self.Health` (`self.Max health`))
  (`self.Update shield material`))

(fn `Enable shield`
  (params (Enabled :type Boolean))
  (`SceneComponent.SetVisibility` (`self.Sphere`) Enabled false)
  (`self.SetActorEnableCollision` Enabled))

(fn `TakeDamage`
  (params (Damage :type "Float (double-precision)"))
  (set `self.Health` (- (`self.Health`) Damage)))

(fn `Update shield material`
  (`MaterialInstanceDynamic.SetScalarParameterValue` (`self.Shield material`) "Shield health" (`KismetMathLibrary.MapRangeClamped` (`self.Health`) 0.0 (`self.Max health`) 0.0 1.0)))

(fn `UserConstructionScript`)