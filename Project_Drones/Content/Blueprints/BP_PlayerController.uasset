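; Player controller for the drone swarm game that routes input to the player drone found in the level.
; Axis inputs move the drone along its own axes and turn the view through controller yaw and pitch.
; Fire buttons set the trigger state and fire the primary and secondary child-actor weapons, while shield input only prints a message.
; Pause toggles the pause widget and game pause, only in one specific game mode state.
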(event `self.ReceiveBeginPlay`
  ;[1 0.773 0] Init
  (bind _asgm_drone_swarm (cast `/Game/Blueprints/GM_DroneSwarm` (`GameplayStatics.GetGameMode`)))
  (set `self.Gamemode ref` _asgm_drone_swarm)
  (bind _returnvalue (`GameplayStatics.GetActorOfClass` "/Game/Blueprints/Actors/Drones/BP_PlayerDrone.BP_PlayerDrone_C"))
  (set `self.Player ref` _returnvalue))

(event `InputAxis|Move left/right`
  (params (AxisValue :type "Float (single-precision)"))
  (bind _player_ref (`self.Player ref`))
  ;[0.217 1 0] Left / right movement
  (`Pawn.AddMovementInput` _player_ref (`self.GetActorRightVector` _player_ref) AxisValue false))

(event `InputAxis|Move forward/backward`
  (params (AxisValue :type "Float (single-precision)"))
  (bind _player_ref (`self.Player ref`))
  ;[0.217 1 0] Foward / backward movement
  (`Pawn.AddMovementInput` _player_ref (`self.GetActorForwardVector` _player_ref) AxisValue false))

(event `InputAxis|Move up/down`
  (params (AxisValue :type "Float (single-precision)"))
  (bind _player_ref (`self.Player ref`))
  ;[0.217 1 0] Up / down movement
  (`Pawn.AddMovementInput` _player_ref (`self.GetActorUpVector` _player_ref) AxisValue false))

(event `InputAxis|Aim left/right`
  (params (AxisValue :type "Float (single-precision)"))
  ;[0.217 1 0] Aiming
  (`Pawn.AddControllerYawInput` (`GameplayStatics.GetPlayerPawn` 0) AxisValue))

(event `InputAxis|Aim up/down`
  (params (AxisValue :type "Float (single-precision)"))
  ;[0.217 1 0] Aiming
  (`Pawn.AddControllerPitchInput` (`GameplayStatics.GetPlayerPawn` 0) AxisValue))

(event `InputAction|Pause` :paused true
  (params (Key :type "Key Structure"))
  ;[0.217 1 0] Game pause
  (:`Pressed`
    (if (`|EnumEquality` (`/Game/Blueprints/GM_DroneSwarm.Game state` (`self.Gamemode ref`)) "NewEnumerator2")
      (if (`GameplayStatics.IsGamePaused`)
        (`Widget.RemoveFromParent` (stale _returnvalue))
        (`GameplayStatics.SetGamePaused` false)
        (else
          (bind _returnvalue (`|CreateWidget` "/Game/UI/UI_Paused.UI_Paused_C"))
          (`UserWidget.AddToViewport` _returnvalue 0)
          (`GameplayStatics.SetGamePaused` true))))))

(event `InputAction|Fire left`
  (params (Key :type "Key Structure"))
  (bind _asbp_weapon_base (cast `/Game/Blueprints/Weapons/BP_WeaponBase` (`ChildActorComponent.ChildActor` (`/Game/Blueprints/Actors/Drones/BP_PlayerDrone.Primary weapon` (`self.Player ref`))) :!pure true))
  ;[0.217 1 0] Fire default weapon
  (:`Pressed`
    (set `/Game/Blueprints/Weapons/BP_WeaponBase.IsTriggerDown?` true _asbp_weapon_base)
    (`/Game/Blueprints/Weapons/BP_WeaponBase.Fire weapon` _asbp_weapon_base)
    (`KismetSystemLibrary.PrintString` "Firing primary weapon!" true true (struct :`R` 1.0 :`G` 0.09667 :`A` 1.0) 0.5))
  (:`Released`
    (set `/Game/Blueprints/Weapons/BP_WeaponBase.IsTriggerDown?` false _asbp_weapon_base)))

(event `InputAction|Fire right`
  (params (Key :type "Key Structure"))
  (bind _asbp_weapon_base (cast `/Game/Blueprints/Weapons/BP_WeaponBase` (`ChildActorComponent.ChildActor` (`/Game/Blueprints/Actors/Drones/BP_PlayerDrone.Secondary weapon` (`self.Player ref`))) :!pure true))
  ;[0.217 1 0] Fire second weapon
  (:`Pressed`
    (set `/Game/Blueprints/Weapons/BP_WeaponBase.IsTriggerDown?` true _asbp_weapon_base)
    (`/Game/Blueprints/Weapons/BP_WeaponBase.Fire weapon` _asbp_weapon_base)
    (`KismetSystemLibrary.PrintString` "Firing secondary weapon!" true true (struct :`R` 1.0 :`G` 0.09667 :`A` 1.0) 0.5))
  (:`Released`
    (set `/Game/Blueprints/Weapons/BP_WeaponBase.IsTriggerDown?` false _asbp_weapon_base)))

(event `InputAction|Activate shield`
  (params (Key :type "Key Structure"))
  ;[0.217 1 0] Activate shield
  (:`Pressed`
    (`KismetSystemLibrary.PrintString` "Shield activated!" true true (struct :`R` 1.0 :`G` 0.09667 :`A` 1.0) 0.5)))

(fn `UserConstructionScript`)