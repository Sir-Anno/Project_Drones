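; BP_MusicManger is a music manager actor that plays the menu track when the drone swarm game mode enters its Menu state.
; On BeginPlay it caches the game mode and game instance and binds to the game mode's new-state dispatcher.
; Playtrack creates and stores a non-auto-destroying 2D sound, which Fademusic can fade in or out.
; Only the Menu state is handled, and nothing here calls Fademusic.
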(event `self.ReceiveBeginPlay`
  (bind _asgm_drone_swarm (cast `/Game/Blueprints/GM_DroneSwarm` (`GameplayStatics.GetGameMode`)))
  (bind _output_get (set `self.Gamemode ref` _asgm_drone_swarm))
  (add `/Game/Blueprints/GM_DroneSwarm.ED_NewGameState` _output_get (`|CreateDelegate` :!event `ED_NewGameState`))
  (bind _asgi_game_instance (cast `/Game/Blueprints/GI_GameInstance` (`GameplayStatics.GetGameInstance`)))
  (set `self.Game instance ref` _asgi_game_instance))

(event `ED_NewGameState`
  (params (`New state` :type "/Game/Blueprints/E_GameStates Enum" :default "NewEnumerator0"))
  (switch `/Game/Blueprints/E_GameStates` `New state`
    (:`NewEnumerator1`
      (`self.Play track` "/Game/Assets/Sounds/Music/SFX_Menu.SFX_Menu"))))

(event `Play track`
  (params (Sound :type "SoundBase Object Reference"))
  (bind _returnvalue (`GameplayStatics.CreateSound2D` Sound 1.0 1.0 0.0 null false false))
  (bind _output_get (set `self.Current track` _returnvalue))
  (`AudioComponent.Play` _output_get 0.0))

(event `Fade music`
  (params (`Fade in?` :type Boolean))
  (if `Fade in?`
    (`AudioComponent.FadeIn` (`self.Current track`) 1.0 1.0 0.0 "Linear")
    (else
      (`AudioComponent.FadeOut` (`self.Current track`) 1.0 0.0 "Linear"))))

(fn `UserConstructionScript`)