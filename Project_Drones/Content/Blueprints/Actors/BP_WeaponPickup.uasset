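; BP_WeaponPickup is a world pickup that equips a weapon in a set slot on the player drone.
; The construction script spawns the chosen Weapon class as a child actor with collision disabled, and BeginPlay puts its name on a widget card.
; Tick billboards that card toward the drone's camera.
; Overlapping the pickup sphere with a drone passes the child weapon to EquipWeapon, then destroys the pickup.
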(event `self.ReceiveBeginPlay`
  (bind _asbp_weapon_base (cast `/Game/Blueprints/Weapons/BP_WeaponBase` (`ChildActorComponent.ChildActor` (`self.Weapon BP`))))
  (bind _returnvalue (`|CreateWidget` "/Game/UI/Custom_Elements/UI_Text.UI_Text_C" null (`.Weaponname_2_BE6D280D4BAB3A83C10E62A224261735` (break `/Game/Blueprints/Weapons/Data/S_WeaponDetails` (`/Game/Blueprints/Weapons/BP_WeaponBase.Weapon stats` _asbp_weapon_base))) "/Game/Assets/Fonts/airstrike_Font.airstrike_Font"))
  (`WidgetComponent.SetWidget` (`self.Weapon card`) _returnvalue))

(event `self.Pickup sphere.OnComponentBeginOverlap`
  (params (OverlappedComponent :type "PrimitiveComponent Object Reference") (OtherActor :type "Actor Object Reference") (OtherComp :type "PrimitiveComponent Object Reference") (OtherBodyIndex :type Integer) (bFromSweep :type Boolean) (SweepResult :type "HitResult Structure (by ref)"))
  (bind _asbp_player_drone (cast `/Game/Blueprints/Actors/Drones/BP_PlayerDrone` OtherActor))
  (`/Game/Blueprints/Actors/Drones/BP_PlayerDrone.EquipWeapon` _asbp_player_drone (`self.Weapon slot`) (cast `/Game/Blueprints/Weapons/BP_WeaponBase` (`ChildActorComponent.ChildActor` (`self.Weapon BP`)) :!pure true))
  (`self.K2_DestroyActor`))

(event `self.ReceiveTick`
  (params (DeltaSeconds :type "Float (single-precision)"))
  (bind _weapon_card (`self.Weapon card`))
  (bind _asbp_player_drone (cast `/Game/Blueprints/Actors/Drones/BP_PlayerDrone` (`GameplayStatics.GetPlayerPawn` 0)))
  (`SceneComponent.K2_SetWorldRotation` _weapon_card (`KismetMathLibrary.FindLookAtRotation` (`SceneComponent.K2_GetComponentLocation` _weapon_card) (`SceneComponent.K2_GetComponentLocation` (`/Game/Blueprints/Actors/Drones/BP_PlayerDrone.Camera` _asbp_player_drone))) false false))

(fn `UserConstructionScript`
  (bind _weapon_bp (`self.Weapon BP`))
  (`ChildActorComponent.SetChildActorClass` _weapon_bp (`self.Weapon`))
  (`self.SetActorEnableCollision` (`ChildActorComponent.ChildActor` _weapon_bp) false))