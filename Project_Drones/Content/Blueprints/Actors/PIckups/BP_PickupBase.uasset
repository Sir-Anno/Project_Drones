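; BP_PickupBase is a pickup actor that adds health to the player drone when it enters the pickup radius, then destroys itself.
; On BeginPlay it creates a UI_Text widget reading "Health" and assigns it to its widget component.
; Every Tick it rotates that widget to face the player camera, billboarding the label.
; Despite the base name, both the label and the effect are health-specific.
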(event `self.ReceiveBeginPlay`
  (bind _returnvalue (`|CreateWidget` "/Game/UI/Custom_Elements/UI_Text.UI_Text_C" null "Health" "/Game/Assets/Fonts/airstrike_Font.airstrike_Font"))
  (set `/Game/UI/Custom_Elements/UI_Text.Font size` 72 _returnvalue)
  (`WidgetComponent.SetWidget` (`self.Widget`) _returnvalue))

(event `self.ReceiveTick`
  (params (DeltaSeconds :type "Float (single-precision)"))
  (`SceneComponent.K2_SetWorldRotation` (`self.Widget`) (`KismetMathLibrary.FindLookAtRotation` (`SceneComponent.K2_GetComponentLocation` (`self.Widget`)) (`PlayerCameraManager.GetCameraLocation` (`GameplayStatics.GetPlayerCameraManager` 0))) false false))

(event `self.PickupRadius.OnComponentBeginOverlap`
  (params (OverlappedComponent :type "PrimitiveComponent Object Reference") (OtherActor :type "Actor Object Reference") (OtherComp :type "PrimitiveComponent Object Reference") (OtherBodyIndex :type Integer) (bFromSweep :type Boolean) (SweepResult :type "HitResult Structure (by ref)"))
  (bind _asbp_player_drone (cast `/Game/Blueprints/Actors/Drones/BP_PlayerDrone` OtherActor))
  (`/Game/Blueprints/Components/C_HealthSystem.Add health` (`/Game/Blueprints/Actors/Drones/BP_Drone_Base.C_HealthSystem` _asbp_player_drone) (`self.Health To Add`))
  (`self.K2_DestroyActor`))

(fn `UserConstructionScript`)