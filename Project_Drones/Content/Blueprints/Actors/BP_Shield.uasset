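; Shield actor attached to a parent drone that absorbs damage and shows its remaining health through a dynamic material parameter.
; Each hit resets the recharge timers; after a delay without damage, a looping timer refills health in steps.
; A depleted shield hides itself, disables collision and returns at full health after a regen delay.
; When the owning drone's killed event fires, pending regen is cancelled and the shield is switched off.
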(event `self.ReceiveBeginPlay`
  (bind _returnvalue (`self.GetParentActor`))
  (`|ExecutionSequence`
    (:`then_0`
      ;[0.1 0.1 0.1] Set reference to attached drone
      (`/Engine/EditorBlueprintResources/StandardMacros.IsValid` _returnvalue
        (:`Is Valid`
          (bind _asbp_drone_base (cast `/Game/Blueprints/Actors/Drones/BP_Drone_Base` _returnvalue))
          (bind _output_get (set `self.Owning drone` _asbp_drone_base))
          (add `/Game/Blueprints/Actors/Drones/BP_Drone_Base.ED_DroneKilled` _output_get (`|CreateDelegate` :!event `ED_DroneKilled`)))))
    (:`then_1`
      ;[0.1 0.1 0.1] Create matieral instance
      (bind _returnvalue_2 (`PrimitiveComponent.CreateDynamicMaterialInstance` (`self.Sphere`) 0 "/Game/Assets/Materials/M_DroneShield.M_DroneShield" "None"))
      (set `self.Shield material` _returnvalue_2))))

(event `self.ReceiveAnyDamage`
  (params (Damage :type "Float (single-precision)") (DamageType :type "DamageType Object Reference") (InstigatedBy :type "Controller Object Reference") (DamageCauser :type "Actor Object Reference"))
  ;[0.1 0.1 0.1] Take damage
  (`self.TakeDamage` Damage)
  (`self.Update shield material`)
  ;;[0.1 0.1 0.1] Reset timers
  (`KismetSystemLibrary.K2_ClearAndInvalidateTimerHandle` (`self.Recharge timer`))
  (`KismetSystemLibrary.K2_ClearAndInvalidateTimerHandle` (`self.Recharge delay timer`))
  (`self.Check shield down`
    (:`Shield down`
      (`self.Enable shield` false)
      (`self.Start shield regen`))
    (:`Shield up`
      (bind _returnvalue (`KismetSystemLibrary.K2_SetTimerDelegate` (`|CreateDelegate` :!event `Start shield recharge`) (`self.Shield recharge delay`))) ; Start shield recharge if no damage has \nbeen taken after shield recharge delay
      (set `self.Recharge delay timer` _returnvalue))))

(event `Start shield recharge`
  ;[0.1 0.1 0.1] Recharge shield if no damage has been taken after shield recharge delay
  (bind _returnvalue (`KismetSystemLibrary.K2_SetTimerDelegate` (delegate `Recharge shield`) (`self.Shield recharge rate`) true))
  (set `self.Recharge timer` _returnvalue))

(event `Recharge shield`
  ;[0.1 0.1 0.1] Recharge shield if no damage has been taken after shield recharge delay
  (set `self.Shield health` (`KismetMathLibrary.FClamp` (+ (`self.Shield health`) (`self.Shield recharge amount`)) 0.0 (`self.Shield max health`)))
  (`self.Update shield material`))

(event `Start shield regen`
  ;[0.1 0.1 0.1] Regen shield after delay
  (bind _returnvalue (`KismetSystemLibrary.K2_SetTimerDelegate` (delegate `Regen shield`) (`self.Shield regen delay`)))
  (set `self.Shield regen timer` _returnvalue))

(event `Regen shield`
  ;[0.1 0.1 0.1] Regen shield after delay
  (set `self.Shield health` (`self.Shield max health`))
  (`self.Enable shield` true)
  (`self.Update shield material`))

(event `ED_DroneKilled`
  (params (`Drone ref` :type "/Game/Blueprints/Actors/Drones/BP_Drone_Base Object Reference"))
  ;[0.1 0.1 0.1] Drone killed
  (`KismetSystemLibrary.K2_ClearAndInvalidateTimerHandle` (`self.Shield regen timer`))
  (`self.Enable shield` false))

(fn `Enable shield`
  (params (Enabled :type Boolean))
  (`SceneComponent.SetVisibility` (`self.Sphere`) Enabled false)
  (`self.SetActorEnableCollision` Enabled))

(fn `TakeDamage`
  (params (Damage :type "Float (double-precision)"))
  (set `self.Shield health` (- (`self.Shield health`) Damage)))

(fn `Update shield material`
  (`MaterialInstanceDynamic.SetScalarParameterValue` (`self.Shield material`) "Shield health" (`KismetMathLibrary.MapRangeClamped` (`self.Shield health`) 0.0 (`self.Shield max health`) 0.0 1.0)))

(fn `UserConstructionScript`
  (set `self.Shield max health` (`self.Shield health`)))