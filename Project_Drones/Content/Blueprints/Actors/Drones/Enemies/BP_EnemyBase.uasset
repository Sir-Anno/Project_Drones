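; Base Blueprint for enemy drones that adds damage feedback and kill scoring on top of its parent's health behavior.
; Any damage runs the parent handler, then spawns a BP_DamageNumbers actor above the drone showing the damage taken.
; On death, a DoOnce guard reports the drone's score to the game mode a single time before calling the parent's killed logic.
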(event `self.ReceiveAnyDamage`
  (params (Damage :type "Float (single-precision)") (DamageType :type "DamageType Object Reference") (InstigatedBy :type "Controller Object Reference") (DamageCauser :type "Actor Object Reference"))
  ;[0.217 1 0] Damage numbers
  (`parent.ReceiveAnyDamage` Damage DamageType InstigatedBy DamageCauser)
  (`self.SpawnDamageNumbers` Damage))

(event `self.ED_HealthKilled`
  ;[0.217 1 0] Drone killed
  (`/Engine/EditorBlueprintResources/StandardMacros.DoOnce` false
    (:`Completed`
      (message `/Game/Blueprints/BPI_EnemyKilled.EnemyKilled` (`self.Gamemode Ref`) (`self.Drone score`))
      (`parent.ED_HealthKilled`))))

(fn `SpawnDamageNumbers`
  (params (`Damage taken` :type "Float (double-precision)"))
  (`|SpawnActorFromClass` "/Game/Blueprints/Actors/BP_DamageNumbers.BP_DamageNumbers_C" (`KismetMathLibrary.MakeTransform` (+ (`self.K2_GetActorLocation`) (0.0 0.0 200.0))) "Undefined" "OverrideRootScale" null `Damage taken` null))

(fn `UserConstructionScript`)