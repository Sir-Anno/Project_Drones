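; Base drone pawn for the drone swarm game mode, with health, an optional shield and optional floating movement.
; The construction script configures all three from DroneStats, removing shield or movement components the stats do not call for.
; Damage goes to the health component, whose update event adds sparks below half health and fire below a third.
; On death it notifies the game mode, falls with physics, then explodes and destroys itself when the fall sound finishes.
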(event `self.ReceiveBeginPlay`
  ;[0.217 1 0] Set up
  (bind _asgm_drone_swarm (cast `/Game/Blueprints/GM_DroneSwarm` (`GameplayStatics.GetGameMode`)))
  (set `self.Gamemode Ref` _asgm_drone_swarm)
  (add `/Game/Blueprints/Components/C_HealthSystem.ED_HealthUpdated` (`self.C_HealthSystem`) (`|CreateDelegate` :!event `ED_HealthUpdated`))
  (add `/Game/Blueprints/Components/C_HealthSystem.ED_Killed` (`self.C_HealthSystem`) (`|CreateDelegate` :!event `ED_HealthKilled`)))

(event `self.ReceiveAnyDamage`
  (params (Damage :type "Float (single-precision)") (DamageType :type "DamageType Object Reference") (InstigatedBy :type "Controller Object Reference") (DamageCauser :type "Actor Object Reference"))
  ;[0.217 1 0] Take damage and death check
  (`/Game/Blueprints/Components/C_HealthSystem.Take damage` (`self.C_HealthSystem`) Damage))

(event `ED_HealthUpdated`
  (params (Health :type "Float (double-precision)") (`Health percentage` :type "Float (double-precision)"))
  ;[0.217 1 0] Health updated and damage effects
  (`self.50% Health damage`)
  (`self.30% Health damage`))

(event `ED_HealthKilled`
  ;[0.217 1 0] Drone destroyed
  (`/Engine/EditorBlueprintResources/StandardMacros.DoOnce` false
    (:`Completed`
      (`self.ED_DroneKilled`)
      (message `/Game/Blueprints/BPI_EnemyKilled.EnemyKilled` (`self.Gamemode Ref`) self 0)
      (`PrimitiveComponent.SetSimulatePhysics` (`self.Mesh`) true)
      (bind _returnvalue (`GameplayStatics.SpawnSoundAttached` "/Game/Assets/Sounds/SFX/Drone_fall.Drone_fall" (`self.Mesh`) "None" (`self.K2_GetActorLocation`) (struct) "KeepRelativeOffset" false 1.0 1.0 0.0 null null))
      (add `AudioComponent.OnAudioFinished` _returnvalue (delegate `Fall sound finished`)))))

(event `Fall sound finished`
  (bind _returnvalue (`self.K2_GetActorLocation`))
  ;[0.217 1 0] Drone destroyed
  (`GameplayStatics.SpawnEmitterAtLocation` "/Game/StarterContent/Particles/P_Explosion.P_Explosion" _returnvalue (struct) (5.0 5.0 5.0))
  (`GameplayStatics.PlaySoundAtLocation` "/Game/Assets/Sounds/SFX/Drone_explosion.Drone_explosion" _returnvalue (struct) 1.0 1.0 0.0 null null null null)
  (`self.K2_DestroyActor`))

(fn `30% Health damage`
  (locals (`Emitter ref` :type "ParticleSystemComponent Object Reference"))
  (bind _c_healthsystem (`self.C_HealthSystem`))
  (if (< (`/Game/Blueprints/Components/C_HealthSystem.Health` _c_healthsystem) (/ (`/Game/Blueprints/Components/C_HealthSystem.MaxHealth` _c_healthsystem) 3))
    (`ParticleSystemComponent.SetTemplate` (`self.FireParticle`) "/Game/StarterContent/Particles/P_Fire.P_Fire")))

(fn `50% Health damage`
  (bind _c_healthsystem (`self.C_HealthSystem`))
  (if (< (`/Game/Blueprints/Components/C_HealthSystem.Health` _c_healthsystem) (/ (`/Game/Blueprints/Components/C_HealthSystem.MaxHealth` _c_healthsystem) 2))
    (`ParticleSystemComponent.SetTemplate` (`self.SparksParticle`) "/Game/StarterContent/Particles/P_Sparks.P_Sparks")))

(fn `Setup health`
  (set `/Game/Blueprints/Components/C_HealthSystem.Health` (`.Health_6_CCDA285843888D4EFE5286A7C659534E` (break `/Game/Blueprints/Actors/Drones/S_DroneStats` (`self.Drone stats`))) (`self.C_HealthSystem`)))

(fn `Setup movement`
  (bind _floatingpawnmovement (`self.FloatingPawnMovement`))
  (bind ((`Maxmovementspeed_9_AE4DCBC3492730757993D4BCE99DEA4B` _maxmovementspeed) (`Accelerationspeed_11_6219009E49D75419EE54F9969F26178F` _accelerationspeed) (`Decelerationspeed_13_3D41D9C44D0EB9C6BA2878A47010808B` _decelerationspeed)) (break `/Game/Blueprints/Actors/Drones/S_DroneStats` (`self.Drone stats`)))
  (if (> _maxmovementspeed 0.0)
    (set `FloatingPawnMovement.MaxSpeed` _maxmovementspeed _floatingpawnmovement)
    (set `FloatingPawnMovement.Acceleration` _accelerationspeed _floatingpawnmovement)
    (set `FloatingPawnMovement.Deceleration` _decelerationspeed _floatingpawnmovement)
    (else
      (`ActorComponent.K2_DestroyComponent` (`self.FloatingPawnMovement`)))))

(fn `Setup shield`
  (bind ((`Hasshield_15_D4C751144CEA56E0F49449A981816D4C` _hasshield) (`Shieldhealth_27_403ED10740E21D52DCFA29B4BC4107B6` _shieldhealth) (`Shieldrechargerate_33_58F66A0F42D24FE6A9FA29A837C4E2F6` _shieldrechargerate) (`Shieldrechargeamount_28_D4A2E75446C57CCF5910D4AD93C448FB` _shieldrechargeamount) (`Shieldrechargedelay_29_EC192FFE4AA15DF2AADB258799B187E4` _shieldrechargedelay) (`Shieldregendelay_30_5FBA260343982EE59DC0A0BDB1B45829` _shieldregendelay)) (break `/Game/Blueprints/Actors/Drones/S_DroneStats` (`self.Drone stats`)))
  (if _hasshield
    (bind _asbp_shield (cast `/Game/Blueprints/Actors/BP_Shield` (`ChildActorComponent.ChildActor` (`self.Shield`))))
    (set `/Game/Blueprints/Actors/BP_Shield.Shield health` _shieldhealth _asbp_shield)
    (set `/Game/Blueprints/Actors/BP_Shield.Shield recharge rate` _shieldrechargerate _asbp_shield)
    (set `/Game/Blueprints/Actors/BP_Shield.Shield recharge amount` _shieldrechargeamount _asbp_shield)
    (set `/Game/Blueprints/Actors/BP_Shield.Shield recharge delay` _shieldrechargedelay _asbp_shield)
    (set `/Game/Blueprints/Actors/BP_Shield.Shield regen delay` _shieldregendelay _asbp_shield)
    (else
      (`ActorComponent.K2_DestroyComponent` (`self.Shield`)))))

(fn `UserConstructionScript`
  ;[0.1 0.1 0.1] Setup drone stats
  (`self.Setup health`)
  (`self.Setup movement`)
  (`self.Setup shield`))