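; Player-controlled drone pawn that aims two child-actor weapons, creates its HUD on possession and signals when the player is killed.
; Each tick, a trace from just below the camera finds a hit or far endpoint, and both weapons rotate toward it.
; The construction script sets the drone as each weapon's owner.
; Debug keys apply self-damage or add score, and an on-screen readout shows velocity and health.
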(event `Key|NumPadZero`
  (params (Key :type "Key Structure"))
  ;[1 0.773 0] Debugging
  (:`Pressed`
    (`GameplayStatics.ApplyDamage` self 20.0)))

(event `Key|NumPadOne`
  (params (Key :type "Key Structure"))
  ;[1 0.773 0] Debugging
  (:`Pressed`
    (bind _asgm_drone_swarm (cast `/Game/Blueprints/GM_DroneSwarm` (`GameplayStatics.GetGameMode`)))
    (`/Engine/EditorBlueprintResources/StandardMacros.IncrementInt` (`/Game/Blueprints/GM_DroneSwarm.Score` _asgm_drone_swarm))))

(event `DebugTick`
  (params (`Delta seconds` :type "Float (double-precision)"))
  ;[1 0.773 0] Debugging
  (`KismetSystemLibrary.PrintString` (`KismetStringLibrary.Concat_StrStr` "Velocity: " (`KismetStringLibrary.Conv_DoubleToString` (`KismetMathLibrary.VSize` (`self.GetVelocity`))) " \nHealth: " (`KismetStringLibrary.Conv_DoubleToString` (`/Game/Blueprints/Components/C_HealthSystem.Health` (`self.C_HealthSystem`)))) true true (struct :`R` 0.217042 :`G` 1.0 :`A` 1.0) `Delta seconds`))

(event `self.ReceiveBeginPlay`
  (bind _returnvalue (`GameplayStatics.GetPlayerCameraManager` 0))
  ;[0.217 1 0] Set up
  (`parent.ReceiveBeginPlay`)
  (set `PlayerCameraManager.ViewPitchMin` -75.0 _returnvalue)
  (set `PlayerCameraManager.ViewPitchMax` 75.0 _returnvalue))

(event `self.ReceiveTick`
  (params (DeltaSeconds :type "Float (single-precision)"))
  ;[0.217 1 0] Aim weapons
  (`self.DebugTick` DeltaSeconds)
  (`self.AimWeapons`))

(event `self.ReceivePossessed`
  (params (NewController :type "Controller Object Reference"))
  (bind _returnvalue (`GameplayStatics.GetPlayerController` 0))
  ;[0.217 1 0] Possessed
  (`KismetSystemLibrary.PrintString` "Player possessed!")
  (`WidgetBlueprintLibrary.SetInputMode_GameOnly` _returnvalue)
  (set `PlayerController.bShowMouseCursor` false _returnvalue)
  (bind _returnvalue_2 (`|CreateWidget` "/Game/UI/UI_HUD.UI_HUD_C" null self))
  (`UserWidget.AddToViewport` _returnvalue_2 0))

(event `self.ED_HealthKilled`
  ;[0.217 1 0] Player killed
  (`parent.ED_HealthKilled`)
  (`KismetSystemLibrary.PrintString` "Player died! :(")
  (`self.ED_PlayerKilled`))

(fn `AimWeapons`
  (locals (`Target location` :type "Vector Structure"))
  (bind _returnvalue (- (`SceneComponent.K2_GetComponentLocation` (`self.Camera`)) (0.0 0.0 50.0)))
  ;[0.217 1 0] Aim weapons at a target in range or at a max weapons range distance if no target is in range
  (bind _outhit (`KismetSystemLibrary.LineTraceSingle` _returnvalue (+ _returnvalue (* (`SceneComponent.GetForwardVector` (`self.Camera`)) 100000.0)) "TraceTypeQuery2" false (`|MakeArray` self :!type "Actor Object Reference") "None" true (struct :`R` 1.0 :`A` 1.0) (struct :`G` 1.0 :`A` 1.0) 0.01)) ; Fire a line trace from the centre of the camera
  (bind (_bblockinghit _binitialoverlap _time _distance _location _impactpoint _normal _impactnormal _physmat _hitactor _hitcomponent _hitbonename _bonename _hititem _elementindex _faceindex _tracestart _traceend) (`GameplayStatics.BreakHitResult` _outhit))
  (if _bblockinghit
    (set `local.Target location` _location) ; If a target is hit set target \nlocation to the location of \nthe trace hit
    (else
      (set `local.Target location` _traceend) ; If no target is hit set target\nlocation to the end of the trace
    ))
  (`SceneComponent.K2_SetWorldRotation` (`self.Primary weapon`) (`KismetMathLibrary.FindLookAtRotation` (`SceneComponent.K2_GetComponentLocation` (`self.Primary weapon`)) (`local.Target location`)) false false) ; Rotate primary weapon \nto face target location
  (`SceneComponent.K2_SetWorldRotation` (`self.Secondary weapon`) (`KismetMathLibrary.FindLookAtRotation` (`SceneComponent.K2_GetComponentLocation` (`self.Secondary weapon`)) (`local.Target location`)) false false) ; Rotate secondary weapon \nto face target location
)

(fn `UserConstructionScript`
  (bind _asbp_weapon_base (cast `/Game/Blueprints/Weapons/BP_WeaponBase` (`ChildActorComponent.ChildActor` (`self.Primary weapon`))))
  (set `/Game/Blueprints/Weapons/BP_WeaponBase.Owning drone` self _asbp_weapon_base)
  (bind _asbp_weapon_base_2 (cast `/Game/Blueprints/Weapons/BP_WeaponBase` (`ChildActorComponent.ChildActor` (`self.Secondary weapon`))))
  (set `/Game/Blueprints/Weapons/BP_WeaponBase.Owning drone` self _asbp_weapon_base_2))