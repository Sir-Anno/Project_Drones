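; BP_ZoneTransition is a transition actor that, while active, carries the player drone along a spline to another area.
; Overlapping EnterPoint disables input and plays a timeline that pulls the drone to the actor's location, then Tick advances it along the spline at Speed.
; Near the spline end it restores input, deactivates and activates the optional WaveToActivate.
; SetActive swaps the mesh between green and red materials, also applied at construction.
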(event `self.Enter point.OnComponentBeginOverlap`
  (params (OverlappedComponent :type "PrimitiveComponent Object Reference") (OtherActor :type "Actor Object Reference") (OtherComp :type "PrimitiveComponent Object Reference") (OtherBodyIndex :type Integer) (bFromSweep :type Boolean) (SweepResult :type "HitResult Structure (by ref)"))
  (bind _player_ref (`self.Player ref`))
  (set `self.Distance` 0.0)
  (if (`self.IsActive?`)
    ;[0.217 1 0] Disable player input
    (bind _asbp_player_drone (cast `/Game/Blueprints/Actors/Drones/BP_PlayerDrone` OtherActor))
    (bind _output_get (set `self.Player ref` _asbp_player_drone))
    (`self.DisableInput` _output_get (`GameplayStatics.GetPlayerController` 0))
    ;[0.217 1 0] Move player into start position
    (bind (_direction _alpha) (`Timeline|Move to start` :!via `PlayFromStart`)
      (:`Update`
        (`self.K2_SetActorLocation` _player_ref (`KismetMathLibrary.VLerp` (`self.K2_GetActorLocation` _player_ref) (`self.K2_GetActorLocation`) _alpha) false false))
      (:`Finished`
        (set `self.Is moving player?` true)
        (`KismetSystemLibrary.PrintString` "Player entered transition!")))))

(event `/Game/Blueprints/Interfaces/BPI_Activate.Activate`
  (`self.SetActive` true))

(event `self.ReceiveTick`
  (params (DeltaSeconds :type "Float (single-precision)"))
  (bind _spline (`self.Spline`))
  (bind _returnvalue (`SplineComponent.GetLocationAtSplinePoint` _spline (`SplineComponent.GetNumberOfSplinePoints` _spline) "World"))
  ;[0.217 1 0] Move player pawn along spline
  (`/Engine/EditorBlueprintResources/StandardMacros.IsValid` (`self.Player ref`)
    (:`Is Valid`
      (if (`self.Is moving player?`)
        (bind _output_get (set `self.Distance` (+ (* DeltaSeconds (`self.Speed`)) (`self.Distance`))))
        (`self.K2_SetActorLocation` (`self.Player ref`) (`SplineComponent.GetLocationAtDistanceAlongSpline` (`self.Spline`) _output_get "World") false false)
        (set `self.Last spline point location` _returnvalue)
        (if (== (`self.K2_GetActorLocation` (`self.Player ref`)) _returnvalue :`ErrorTolerance` 50.0)
          (set `self.Is moving player?` false)
          (`self.EnableInput` (`self.Player ref`) (`GameplayStatics.GetPlayerController` 0))
          (`self.SetActive` false)
          (`KismetSystemLibrary.PrintString` "Player left transition")
          (bind _wave_to_activate (`self.Wave to activate`)
            (:`then`
              (`/Game/Blueprints/Interfaces/BPI_Activate.Activate` _wave_to_activate))
            (:`else`)))))))

(fn `SetActive`
  (params (`Active?` :type Boolean))
  (bind _staticmesh (`self.StaticMesh`))
  (bind _output_get (set `self.IsActive?` `Active?`))
  (if _output_get
    (`PrimitiveComponent.SetMaterial` _staticmesh 0 "/Game/Assets/Materials/MI_ColourGreen.MI_ColourGreen")
    (else
      (`PrimitiveComponent.SetMaterial` _staticmesh 0 "/Game/Assets/Materials/MI_ColourRed.MI_ColourRed"))))

(fn `UserConstructionScript`
  (`self.SetActive` (`self.IsActive?`)))