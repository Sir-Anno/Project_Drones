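; Camera position actor that hosts a menu widget and blends the player's view between linked menus.
; On BeginPlay it binds to its UI_MenuBase dispatcher, which supplies an index into LinkedMenus.
; A move disables its own collision, enables the target's, and calls SetViewTargetWithBlend on the target.
; After a delay matching the blend time, it signals the target's widget to become the active menu.
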(event `self.ReceiveBeginPlay`
  (bind _asui_menu_base (cast `/Game/UI/UI_MenuBase` (`WidgetComponent.GetUserWidgetObject` (`self.Widget`))))
  (add `/Game/UI/UI_MenuBase.ED_MoveToLinkedMenu` _asui_menu_base (delegate `ED_MoveToLinkedMenu`)))

(event `ED_MoveToLinkedMenu`
  (params (`Menu index` :type Integer))
  (if (`KismetArrayLibrary.Array_IsValidIndex` (`self.Linked menus`) `Menu index`)
    (`self.Move to linked camera` (`|GetArrayItem` (`self.Linked menus`) `Menu index`) 1.0 "VTBlend_EaseInOut" 5.0)))

(event `Move to linked camera`
  (params (`Linked menu` :type "/Game/Blueprints/Actors/BP_CameraPosition Object Reference") (BlendTime :type "Float (single-precision)" :default 2.0) (BlendFunc :type "EViewTargetBlendFunction Enum" :default "VTBlend_EaseInOut") (BlendExp :type "Float (single-precision)" :default 2.0))
  (`self.SetActorEnableCollision` false)
  (`self.SetActorEnableCollision` `Linked menu` true)
  (`PlayerController.SetViewTargetWithBlend` (`GameplayStatics.GetPlayerController` 0) `Linked menu` BlendTime BlendFunc BlendExp false)
  (`KismetSystemLibrary.Delay` BlendTime)
  (bind _asui_menu_base (cast `/Game/UI/UI_MenuBase` (`WidgetComponent.GetWidget` (`/Game/Blueprints/Actors/BP_CameraPosition.Widget` `Linked menu`))))
  (`/Game/UI/UI_MenuBase.ED_SetActiveMenu` _asui_menu_base))

(fn `UserConstructionScript`)