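; Wave spawner actor that runs countdown-led waves of enemy drones and activates a transition zone once all are defeated.
; Activation starts a looping one-second timer driving a countdown widget, then spawns the drone types and counts from the wave-numbered DataTable row at random spawners.
; Kill dispatchers remove drones from the tracked list; when empty, the next wave starts, or a missing row signals completion and resets the wave number.
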(event `self.ReceiveTick`
  (params (DeltaSeconds :type "Float (single-precision)"))
  ;[1 0.9648 0] Debug
  (`KismetSystemLibrary.PrintText` (`|FormatText` "Drones left: {Ammount}" (`KismetArrayLibrary.Array_Length` (`self.Current enemies`))) true true (struct :`G` 0.66 :`B` 1.0 :`A` 1.0) DeltaSeconds))

(event `/Game/Blueprints/Interfaces/BPI_Activate.Activate`
  ;[0.1 0.1 0.1] Wave count down
  (bind _returnvalue (`KismetSystemLibrary.K2_SetTimerDelegate` (delegate `Count down`) 1.0 true :!label _label))
  (set `self.WaveStartsInTime` 3)
  (bind _returnvalue_2 (`|CreateWidget` "/Game/UI/UI_WaveCountDown.UI_WaveCountDown_C"))
  (bind _output_get (set `self.Wave countdown UI` _returnvalue_2))
  (`UserWidget.AddToViewport` _output_get 0))

(event `Start count down`
  ;[0.1 0.1 0.1] Wave count down
  (goto _label))

(event `Count down`
  (bind _wavestartsintime (`self.WaveStartsInTime`))
  ;[0.1 0.1 0.1] Wave count down
  (`/Game/UI/UI_WaveCountDown.Update countdown` (`self.Wave countdown UI`) (`self.WaveStartsInTime`))
  (`/Engine/EditorBlueprintResources/StandardMacros.DecrementInt` _wavestartsintime
    (:`  `
      (if (== _wavestartsintime 0)
        (`KismetSystemLibrary.K2_ClearAndInvalidateTimerHandle` (stale `/Game/Blueprints/Interfaces/BPI_Activate.Activate` _returnvalue))
        (`KismetSystemLibrary.Delay` 1.0)
        (`/Game/UI/UI_WaveCountDown.Set wave text` (`self.Wave countdown UI`) "")
        (`self.SpawnWave`)))))

(event `SpawnWave`
  (bind _returnvalue (`|GetDataTableRow` (`self.WaveDataTable`) (`KismetStringLibrary.Conv_StringToName` (`KismetStringLibrary.Conv_IntToString` (`self.CurrentWave`))))
    (:`then`
      (for _array_element (`.Dronedata_3_8A0E28E74968F1E7EDD53AAC507DCF25` (break `/Game/Blueprints/Actors/WaveSpawner/S_WaveData` _returnvalue))
        (bind (_dronetype _droneammount) (break `/Game/Blueprints/Actors/WaveSpawner/S_DroneData` _array_element))
        (for _ (range 1 (+ _droneammount 1))
          (bind _output_get (`self.PickSpawner`))
          (bind (_returnvalue_location _returnvalue_rotation) (`KismetMathLibrary.BreakTransform` (`self.GetTransform` _output_get)))
          (bind _returnvalue_2 (`|SpawnActorFromClass` _dronetype (`KismetMathLibrary.MakeTransform` _returnvalue_location _returnvalue_rotation (3.0 3.0 3.0)) "AdjustIfPossibleButAlwaysSpawn" "OverrideRootScale" null null))
          (`KismetArrayLibrary.Array_Add` (`self.Current enemies`) _returnvalue_2)
          (add `/Game/Blueprints/Actors/Drones/BP_Drone_Base.ED_DroneKilled` _returnvalue_2 (delegate `Remove drone from current enemies`)))))))

(event `Remove drone from current enemies`
  (params (`Drone ref` :type "/Game/Blueprints/Actors/Drones/BP_Drone_Base Object Reference"))
  (bind _current_enemies (`self.Current enemies`))
  (`KismetArrayLibrary.Array_RemoveItem` _current_enemies `Drone ref`)
  (if (== (`KismetArrayLibrary.Array_Length` _current_enemies) 0)
    (`/Engine/EditorBlueprintResources/StandardMacros.IncrementInt` (`self.CurrentWave`)
      (:`  `
        (bind _returnvalue (`|CreateWidget` "/Game/UI/UI_WaveCountDown.UI_WaveCountDown_C"))
        (`UserWidget.AddToViewport` _returnvalue 0)
        (`self.Check all waves defeated`
          (:`Waves remaining`
            (`/Game/UI/UI_WaveCountDown.Set wave text` _returnvalue "New wave starting!")
            (`KismetSystemLibrary.Delay` 2.0)
            (`self.Start count down`))
          (:`Waves defeated`
            (`/Game/UI/UI_WaveCountDown.Set wave text` _returnvalue "All waves defeated!")
            (`/Game/Blueprints/Interfaces/BPI_Activate.Activate` (`self.Transition zone`))
            (`self.ResetWaves`)))))))

(fn `PickSpawner`
  (returns (Output_Get :type "/Game/Blueprints/Actors/WaveSpawner/BP_WaveSpawnPoint Object Reference"))
  (locals (DroneSpawner :type "/Game/Blueprints/Actors/WaveSpawner/BP_WaveSpawnPoint Object Reference"))
  (bind _output_get (set `local.DroneSpawner` (`KismetArrayLibrary.Array_Random` (`self.Spawners`))))
  (return _output_get))

(fn `ResetWaves`
  (set `self.CurrentWave` 1))

(fn `UserConstructionScript`)