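; Actor that shows a floating damage number through a UI_DamageNumbers widget component.
; Construction offsets it randomly along its local Y axis so numbers spawned together spread out.
; On BeginPlay it passes its DamageValue to the widget and binds to the widget's done event, then destroys itself when that fires.
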(event `self.ReceiveBeginPlay`
  (bind _asui_damage_numbers (cast `/Game/UI/UI_DamageNumbers` (`WidgetComponent.GetWidget` (`self.Widget`))))
  (set `/Game/UI/UI_DamageNumbers.Damage value` (`self.Damage value`) _asui_damage_numbers)
  (add `/Game/UI/UI_DamageNumbers.ED_DamageNumbersDone` _asui_damage_numbers (delegate `ED_DamageNumbersDone`)))

(event `ED_DamageNumbersDone`
  (`self.K2_DestroyActor`))

(fn `UserConstructionScript`
  (`self.K2_AddActorLocalOffset` (`KismetMathLibrary.MakeVector` 0.0 (`KismetMathLibrary.RandomFloatInRange` -150.0 150.0))))