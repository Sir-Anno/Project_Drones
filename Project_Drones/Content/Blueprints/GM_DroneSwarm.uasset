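; Game mode for a drone swarm game that runs the session from menu through play to game over and restart.
; A state switch broadcasts each new state and runs its handler: Setup possesses the player drone after a camera delay, and Quit fades the screen, then reopens the level.
; The player drone's death event triggers a delayed game over screen, while enemy kills update the kill count and score.
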(event `self.ReceiveBeginPlay`
  ;[0.1 0.1 0.1] Init
  (`self.Switch game state` "NewEnumerator1")
  (bind _asbp_player_drone (cast `/Game/Blueprints/Actors/Drones/BP_PlayerDrone` (`GameplayStatics.GetPlayerPawn` 0)))
  (bind _output_get (set `self.Player ref` _asbp_player_drone))
  (add `/Game/Blueprints/Actors/Drones/BP_PlayerDrone.ED_PlayerKilled` _output_get (`|CreateDelegate` :!event `ED_PlayerKilled`))
  (bind _returnvalue (`GameplayStatics.GetActorOfClass` "/Game/Blueprints/Actors/BP_MusicManger.BP_MusicManger_C"))
  (set `self.Music manager ref` _returnvalue))

(event `Switch game state`
  (params (`New state` :type "/Game/Blueprints/E_GameStates Enum" :default "NewEnumerator0"))
  ;[0.1 0.1 0.1] Switch game state
  (`self.ED_NewGameState` `New state`)
  (bind _output_get (set `self.Game state` `New state`))
  (switch `/Game/Blueprints/E_GameStates` _output_get
    (:`NewEnumerator1`
      (`self.Menu`))
    (:`NewEnumerator0`
      (`self.Setup`))
    (:`NewEnumerator3`
      (`self.Game start`))
    (:`NewEnumerator2`
      (`self.In game`))
    (:`NewEnumerator4`
      (`self.Game over`))
    (:`NewEnumerator6`
      (`self.Quit`))
    (:`NewEnumerator7`
      (`self.Restart game`))))

(event `Setup`
  ;[0.1 0.1 0.1] Setup
  (`KismetSystemLibrary.Delay` 1.0) ; Wait for camera transition from main menu
  (bind _returnvalue (`GameplayStatics.GetActorOfClass` "/Game/Blueprints/Actors/Drones/BP_PlayerDrone.BP_PlayerDrone_C"))
  (`Controller.Possess` (`GameplayStatics.GetPlayerController` 0) _returnvalue)
  (`self.Switch game state` "NewEnumerator3"))

(event `Menu`
  ;[0.1 0.1 0.1] Menu
)

(event `Game start`
  ;[0.1 0.1 0.1] Game start
  (`self.Switch game state` "NewEnumerator2"))

(event `In game`
  ;[0.1 0.1 0.1] In game
)

(event `Game over`
  (bind _returnvalue (`GameplayStatics.GetPlayerController` 0))
  ;[0.1 0.1 0.1] Game over
  (`self.DisableInput` _returnvalue _returnvalue)
  (`WidgetBlueprintLibrary.SetInputMode_UIOnlyEx` _returnvalue null)
  (set `PlayerController.bShowMouseCursor` true _returnvalue)
  (bind _returnvalue_2 (`|CreateWidget` "/Game/UI/UI_GameOver.UI_GameOver_C"))
  (`UserWidget.AddToViewport` _returnvalue_2 0))

(event `Quit`
  ;[0.1 0.1 0.1] Quit game
  (bind _returnvalue (`|CreateWidget` "/Game/UI/UI_ScreenFade.UI_ScreenFade_C"))
  (`UserWidget.AddToViewport` _returnvalue 0)
  (bind _fade (`/Game/UI/UI_ScreenFade.Fade` _returnvalue))
  (`UserWidget.PlayAnimation` _returnvalue _fade 0.0 1 "Reverse" 1.0 false)
  (`UserWidget.BindToAnimationFinished` _returnvalue _fade (delegate `Fade finished`)))

(event `Fade finished`
  ;[0.1 0.1 0.1] Quit game
  (`self.Switch game state` "NewEnumerator7"))

(event `Restart game`
  ;[0.1 0.1 0.1] Restart game
  (`GameplayStatics.OpenLevelBySoftObjectPtr` "/Game/Levels/Level.Level"))

(event `ED_PlayerKilled`
  ;[0.1 0.1 0.1] Player killed bind
  (`KismetSystemLibrary.Delay` 2.0)
  (`self.Switch game state` "NewEnumerator4"))

(event `/Game/Blueprints/BPI_EnemyKilled.EnemyKilled`
  (params (`Drone killed` :type "/Game/Blueprints/Actors/Drones/BP_Drone_Base Object Reference") (`Drone score` :type Integer))
  ;[0.1 0.1 0.1] Enemy killed
  (if true
    (`/Engine/EditorBlueprintResources/StandardMacros.IncrementInt` (`self.Drones killed`)
      (:`  `
        (`self.UpdateScore` `Drone score`)))))

(fn `UpdateScore`
  (params (`Points to add` :type Integer))
  (set `self.Score` (+ (`self.Score`) `Points to add`)))

(fn `UserConstructionScript`)