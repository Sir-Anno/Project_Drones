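; Homing missile projectile that seeks the player pawn and explodes on overlap or when shot down.
; On BeginPlay it homes its ProjectileMovement on the player's component tagged HomingTarget, and delays switching its mesh to WorldDynamic as a hack against colliding with its shooter.
; Sphere overlap applies damage, then plays explosion effects and destroys the actor.
; Any damage received destroys it, and the Destroyed event reuses the same explosion path.
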(event `self.ReceiveBeginPlay`
  (`|ExecutionSequence`
    (:`then_0`
      (for _array_element (`self.GetComponentsByTag` (`GameplayStatics.GetPlayerPawn` 0) "/Script/Engine.SceneComponent" "HomingTarget")
        (bind _asscene_component (cast `SceneComponent` _array_element))
        (set `ProjectileMovementComponent.HomingTargetComponent` _asscene_component (`self.ProjectileMovement`))))
    (:`then_1`
      ;[0.1 0.1 0.1] Hack for preventing coliding with the actor that shot it
      (`KismetSystemLibrary.Delay` 0.2)
      (`PrimitiveComponent.SetCollisionObjectType` (`self.StaticMesh`) "ECC_WorldDynamic"))))

(event `self.Sphere.OnComponentBeginOverlap`
  (params (OverlappedComponent :type "PrimitiveComponent Object Reference") (OtherActor :type "Actor Object Reference") (OtherComp :type "PrimitiveComponent Object Reference") (OtherBodyIndex :type Integer) (bFromSweep :type Boolean) (SweepResult :type "HitResult Structure (by ref)"))
  (bind _returnvalue (`self.K2_GetActorLocation`))
  (`GameplayStatics.ApplyDamage` OtherActor 100.0)
  (`GameplayStatics.SpawnEmitterAtLocation` "/Game/StarterContent/Particles/P_Explosion.P_Explosion" _returnvalue :!label _label)
  (`GameplayStatics.PlaySoundAtLocation` "/Game/Assets/Sounds/SFX/Explosion.Explosion" _returnvalue (struct) 1.0 1.0 0.0 null null null null)
  (`self.K2_DestroyActor`))

(event `self.ReceiveDestroyed`
  (goto _label))

(event `self.ReceiveAnyDamage`
  (params (Damage :type "Float (single-precision)") (DamageType :type "DamageType Object Reference") (InstigatedBy :type "Controller Object Reference") (DamageCauser :type "Actor Object Reference"))
  (`self.K2_DestroyActor`))

(fn `UserConstructionScript`)