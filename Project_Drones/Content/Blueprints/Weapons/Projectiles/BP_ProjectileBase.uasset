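; BP_ProjectileBase is a base weapon projectile configured by a ProjectileDetails struct.
; The construction script applies the struct's mesh, trail effect and initial speed to the components and sets the mesh scale.
; On mesh hit it deals kinetic damage to the hit actor with its owner as causer, spawns an impact particle and a surface-aligned temporary decal, then destroys itself.
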(event `self.Mesh.OnComponentHit`
  (params (HitComponent :type "PrimitiveComponent Object Reference") (OtherActor :type "Actor Object Reference") (OtherComp :type "PrimitiveComponent Object Reference") (NormalImpulse :type "Vector Structure") (Hit :type "HitResult Structure (by ref)"))
  (bind (_bblockinghit _binitialoverlap _time _distance _location _impactpoint _normal _impactnormal _physmat _hitactor _hitcomponent) (`GameplayStatics.BreakHitResult` Hit))
  (`GameplayStatics.ApplyDamage` OtherActor (`.Damage_13_B34669C145470AB916B940A6B44E6466` (break `/Game/Blueprints/Weapons/Projectiles/S_ProjectileDetails` (`self.Projectile details`))) null (`self.GetOwner`) "/Game/Blueprints/Weapons/DamageTypes/DT_Kinetic.DT_Kinetic_C")
  (`GameplayStatics.SpawnEmitterAtLocation` (`.Hitparticle_21_516A41FE446A83E2630FAF84DA5A5DE0` (break `/Game/Blueprints/Weapons/Projectiles/S_ProjectileDetails` (`self.Projectile details`))) _location (struct) (2.0 2.0 2.0))
  (`GameplayStatics.SpawnDecalAttached` (`.Hitdecal_24_351325BC4F86C17A2D9545A01FA272AF` (break `/Game/Blueprints/Weapons/Projectiles/S_ProjectileDetails` (`self.Projectile details`))) (64.0 64.0 64.0) _hitcomponent "None" _location (`KismetMathLibrary.Conv_VectorToRotator` _impactnormal) "KeepWorldPosition" 10.0)
  (`self.K2_DestroyActor`))

(fn `UserConstructionScript`
  (bind ((`Projectilemesh_11_473C59144802C04FAA252ABCF2B67943` _projectilemesh) (`Projectiletrail_12_AB60A64542FA9D9B78B7378C2A180024` _projectiletrail) (`Velocity_14_3E1BE16E4DD69B5658314CAADCF90B4E` _velocity)) (break `/Game/Blueprints/Weapons/Projectiles/S_ProjectileDetails` (`self.Projectile details`)))
  (`StaticMeshComponent.SetStaticMesh` (`self.Mesh`) _projectilemesh)
  (`SceneComponent.SetRelativeScale3D` (`self.Mesh`) (`self.Scale`))
  (`ParticleSystemComponent.SetTemplate` (`self.Projectile trail`) _projectiletrail)
  (set `ProjectileMovementComponent.InitialSpeed` _velocity (`self.ProjectileMovement`)))