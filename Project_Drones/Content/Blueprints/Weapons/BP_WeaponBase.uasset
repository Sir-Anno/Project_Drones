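; Base weapon for drones that fires laser or projectile shots from a stats struct, supporting bursts, multi-pellet spread and full-auto.
; FireWeapon runs a delayed, breakable loop per trigger pull, then waits out the fire rate.
; Lasers line-trace for damage and decals, while projectiles spawn actors.
; Event dispatchers broadcast ammo and weapon state; empty magazines refill instantly only with infinite ammo, and the construction script tints the mesh.
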(event `self.ReceiveBeginPlay`
  (`self.ED_WeaponState` "NewEnumerator0")
  (`self.Reload` false))

(event `Fire weapon`
  (bind ((`Shotspertriggerpull_41_9CBFC18E464D37D2F1BF549F7902A407` _shotspertriggerpull) (`Burstdelay_53_606BEFB54C8CED653843FAA211B4318F` _burstdelay)) (break `/Game/Blueprints/Weapons/Data/S_WeaponDetails` (`self.Weapon stats`)))
  (if (`self.IsTriggerDown?`)
    (if (`self.CanFire?`)
      (set `self.CanFire?` false)
      (`/Game/Blueprints/CustomMacros/CustomMacroLibrary.For loop with break with delay` 1 _shotspertriggerpull _burstdelay :!label _label
        (:`Loop body`
          (`self.Check has ammo`
            (:`Has ammo`
              ;[0.217 1 0] Fire corisponding weapon type
              (switch `/Game/Blueprints/Weapons/Data/E_WeaponType` (`.Weapontype_24_157B75194E8C73063A3B9F8FF6F91AA1` (break `/Game/Blueprints/Weapons/Data/S_WeaponDetails` (`self.Weapon stats`)))
                (:`NewEnumerator0`
                  (`self.Shoot laser`))
                (:`NewEnumerator4`
                  (`self.Shoot projectile`)))
              ;[0.217 1 0] Muzzle flash
              (`GameplayStatics.SpawnEmitterAtLocation` (`.Muzzleflash_14_BB9FF5274E9F691E437DE2BEE11EAEA9` (break `/Game/Blueprints/Weapons/Data/S_WeaponDetails` (`self.Weapon stats`))) (`SceneComponent.K2_GetComponentLocation` (`self.Firepoint`)))
              ;[0.217 1 0] Shot sound
              (`GameplayStatics.PlaySoundAtLocation` (`.Shotsound_17_056477F84AD8A0E27CE37C81AFA7FF79` (break `/Game/Blueprints/Weapons/Data/S_WeaponDetails` (`self.Weapon stats`))) (`SceneComponent.K2_GetComponentLocation` (`self.Firepoint`)) (struct) 1.0 1.0 0.0 null null null null)
              ;[0.217 1 0] Reduce ammo count
              (bind _result (`/Engine/EditorBlueprintResources/StandardMacros.DecrementInt` (`self.Ammo count`))
                (:`  `
                  (`self.ED_AmmoCount` _result)
                  (`self.Check has ammo`
                    (:`Out of ammo`
                      (`self.Out of ammo`))))))
            (:`Out of ammo`
              (`self.Break fire loop`)
              (`self.Out of ammo`))))
        (:`Complete`
          ;[0.217 1 0] Delay between shots
          (`KismetSystemLibrary.Delay` (`.Firerate_20_EE9BFD54441DB6F195344CA98964A269` (break `/Game/Blueprints/Weapons/Data/S_WeaponDetails` (`self.Weapon stats`))))
          (set `self.CanFire?` true)
          ;[0.217 1 0] Is fully automatic
          (if (`.Isfullyautomatic?_51_B60C0EFF4D976706F0E2CA8932DCA183` (break `/Game/Blueprints/Weapons/Data/S_WeaponDetails` (`self.Weapon stats`)))
            (`self.Fire weapon`)))))))

(event `Break fire loop`
  (goto _label :!via `Break`))

(event `Out of ammo`
  ;[0.217 1 0] When out of ammo reload
  (if (`.Infiniteammo?_55_2217B1C04564ACCA2A3CF9B0CE35F158` (break `/Game/Blueprints/Weapons/Data/S_WeaponDetails` (`self.Weapon stats`)))
    (`self.Reload` true)
    (set `self.CanFire?` true)
    (`self.Fire weapon`)
    (else
      (`self.ED_WeaponState` "NewEnumerator8"))))

(fn `Shoot laser`
  (bind _returnvalue (`SceneComponent.K2_GetComponentLocation` (`self.Firepoint`)))
  (for _ (range 1 (+ (`.ShotAmmountInShell_65_E809FEE2445CE62EE4AF30AA000E7242` (break `/Game/Blueprints/Weapons/Data/S_WeaponDetails` (`self.Weapon stats`))) 1))
    (bind _outhit (`KismetSystemLibrary.LineTraceSingle` _returnvalue (+ _returnvalue (* (`KismetMathLibrary.RandomUnitVectorInConeInDegrees` (`SceneComponent.GetForwardVector` (`self.Firepoint`)) (`.ShotAccuracyInDegrees_68_0DFA8697436D37E24F608AAD3741C17D` (break `/Game/Blueprints/Weapons/Data/S_WeaponDetails` (`self.Weapon stats`)))) 100000.0)) "TraceTypeQuery3" false (`self.GetAllChildActors` (`self.GetParentActor`) true) "ForDuration" true (struct :`R` 1.0 :`A` 1.0) (struct :`G` 1.0 :`A` 1.0) 0.1))
    (bind (_bblockinghit _binitialoverlap _time _distance _location _impactpoint _normal _impactnormal _physmat _hitactor _hitcomponent) (`GameplayStatics.BreakHitResult` _outhit))
    (`GameplayStatics.ApplyDamage` _hitactor (`.Damage_7_FCA8DC5A4A54A0DF809E23A3F0A4C30A` (break `/Game/Blueprints/Weapons/Data/S_WeaponDetails` (`self.Weapon stats`))) null (`self.Owning drone`) "/Game/Blueprints/Weapons/DamageTypes/DT_Laser.DT_Laser_C")
    (`GameplayStatics.SpawnDecalAttached` "/Game/Assets/Materials/M_LaserHitDecal.M_LaserHitDecal" (64.0 64.0 64.0) _hitcomponent "None" _location (`KismetMathLibrary.Conv_VectorToRotator` _impactnormal) "KeepWorldPosition" 10.0)))

(fn `Shoot projectile`
  (bind _firepoint (`self.Firepoint`))
  (bind _owning_drone (`self.Owning drone`))
  (bind _returnvalue_location (`KismetMathLibrary.BreakTransform` (`SceneComponent.K2_GetComponentToWorld` _firepoint)))
  (for _ (range 1 (+ (`.ShotAmmountInShell_65_E809FEE2445CE62EE4AF30AA000E7242` (break `/Game/Blueprints/Weapons/Data/S_WeaponDetails` (`self.Weapon stats`))) 1))
    (`|SpawnActorFromClass` (`.Projectiletype_60_694AA2394781A88045CA428E425A68B1` (break `/Game/Blueprints/Weapons/Data/S_WeaponDetails` (`self.Weapon stats`))) (`KismetMathLibrary.MakeTransform` _returnvalue_location (`KismetMathLibrary.MakeRotFromX` (`KismetMathLibrary.RandomUnitVectorInConeInDegrees` (`SceneComponent.GetForwardVector` _firepoint) (`.ShotAccuracyInDegrees_68_0DFA8697436D37E24F608AAD3741C17D` (break `/Game/Blueprints/Weapons/Data/S_WeaponDetails` (`self.Weapon stats`)))))) "AlwaysSpawn" "OverrideRootScale" _owning_drone _owning_drone)))

(fn `UserConstructionScript`
  (`MeshComponent.SetVectorParameterValueOnMaterials` (`self.Weapon mesh`) "BodyColor" (`KismetMathLibrary.Conv_LinearColorToVector` (`self.Weapon colour`))))